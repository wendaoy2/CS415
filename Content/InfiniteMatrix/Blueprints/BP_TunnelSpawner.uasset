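; BP_TunnelSpawner builds a chained tunnel of BP_Tunnel segments, populated with enemies and medical pickups.
; On BeginPlay it clears existing tunnels, seeds one at the player, then extends from the newest segment's SpawnPoint.
; Each new segment randomizes its walls and receives a spawner reference.
; Each extension call adds two segments, with random enemy and medic spawns, the medics kept within a circular cross-section by rejection checks.
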(event `self.ReceiveBeginPlay`
  (`self.SpawnInitialTunnels`))

(fn `EnemySpawn`
  (bind _returnvalue_x (`KismetMathLibrary.BreakVector` (`SceneComponent.K2_GetComponentLocation` (`/Game/InfiniteMatrix/Blueprints/BP_Tunnel.SpawnPoint` (`self.Newset Tunnel`)))))
  (if (<= (`KismetMathLibrary.RandomFloat`) 0.75)
    (set `self.LocY` (`KismetMathLibrary.RandomFloatInRange` -300.0 300.0))
    (set `self.LocZ` (`KismetMathLibrary.RandomFloatInRange` -300.0 300.0))
    (`|SpawnActorFromClass` "/Game/InfiniteMatrix/Blueprints/enemy.enemy_C" (`KismetMathLibrary.MakeTransform` (`KismetMathLibrary.MakeVector` (+ _returnvalue_x (`KismetMathLibrary.RandomFloatInRange` 200.0 2300.0)) (`self.LocY`) (`self.LocZ`))) "Undefined" "MultiplyWithRoot" null null)))

(fn `Medic1Spawn`
  (bind _returnvalue_x (`KismetMathLibrary.BreakVector` (`SceneComponent.K2_GetComponentLocation` (`/Game/InfiniteMatrix/Blueprints/BP_Tunnel.SpawnPoint` (`self.Newset Tunnel`)))))
  (set `self.LocZ` (`KismetMathLibrary.RandomFloatInRange` -500.0 500.0))
  (set `self.LocY` (`KismetMathLibrary.RandomFloatInRange` -500.0 500.0))
  (if (<= (+ (`KismetMathLibrary.MultiplyMultiply_FloatFloat` (`self.LocY`) 2.0) (`KismetMathLibrary.MultiplyMultiply_FloatFloat` (`self.LocZ`) 2.0)) 170000.0)
    (`|SpawnActorFromClass` "/Game/InfiniteMatrix/Blueprints/medical.medical_C" (`KismetMathLibrary.MakeTransform` (`KismetMathLibrary.MakeVector` (+ _returnvalue_x (`KismetMathLibrary.RandomFloatInRange` 250.0 2350.0)) (`self.LocY`) (`self.LocZ`))) "Undefined" "MultiplyWithRoot" null null)))

(fn `Medic2Spawn`
  (bind _returnvalue_x (`KismetMathLibrary.BreakVector` (`SceneComponent.K2_GetComponentLocation` (`/Game/InfiniteMatrix/Blueprints/BP_Tunnel.SpawnPoint` (`self.Newset Tunnel`)))))
  (set `self.LocZ` (`KismetMathLibrary.RandomFloatInRange` -500.0 500.0))
  (set `self.LocY` (`KismetMathLibrary.RandomFloatInRange` -500.0 500.0))
  (if (<= (+ (`KismetMathLibrary.MultiplyMultiply_FloatFloat` (`self.LocY`) 2.0) (`KismetMathLibrary.MultiplyMultiply_FloatFloat` (`self.LocZ`) 2.0)) 150000.0)
    (if (<= (`KismetMathLibrary.RandomFloatInRange` 0.0 1.0) 0.5)
      (`|SpawnActorFromClass` "/Game/InfiniteMatrix/Blueprints/medic2.medic2_C" (`KismetMathLibrary.MakeTransform` (`KismetMathLibrary.MakeVector` (+ _returnvalue_x (`KismetMathLibrary.RandomFloatInRange` 200.0 2300.0)) (`self.LocY`) (`self.LocZ`))) "Undefined" "MultiplyWithRoot" null null))))

(fn `SpawnInitialTunnels`
  (`|ExecutionSequence`
    (:`then_0`
      (bind _outactors (`GameplayStatics.GetAllActorsOfClass` "/Game/InfiniteMatrix/Blueprints/BP_Tunnel.BP_Tunnel_C"))
      (for _array_element _outactors
        (`self.K2_DestroyActor` _array_element)))
    (:`then_1`
      (for _ (range 3)
        (`/Engine/EditorBlueprintResources/StandardMacros.IsValid` (`self.Newset Tunnel`)
          (:`Is Valid`
            (`self.SpawnTunnelAtSpawnPoint`))
          (:`Is Not Valid`
            (`self.SpawnTunnel` (`self.K2_GetActorLocation` (`GameplayStatics.GetPlayerPawn` 0)))))))))

(fn `SpawnTunnel`
  (params (SpawnLocation :type "Vector Structure"))
  (bind _returnvalue (`|SpawnActorFromClass` "/Game/InfiniteMatrix/Blueprints/BP_Tunnel.BP_Tunnel_C" (`KismetMathLibrary.MakeTransform` SpawnLocation) "Undefined" "MultiplyWithRoot" null null))
  (bind _output_get (set `self.Newset Tunnel` _returnvalue))
  (set `/Game/InfiniteMatrix/Blueprints/BP_Tunnel.Tunnel Spawner` self _output_get)
  (`/Game/InfiniteMatrix/Blueprints/BP_Tunnel.RandomizeWall` _output_get))

(fn `SpawnTunnelAtSpawnPoint`
  (`self.EnemySpawn`)
  (`|ExecutionSequence`
    (:`then_0`
      (`self.Medic1Spawn`))
    (:`then_1`
      (`self.Medic2Spawn`)))
  (`self.SpawnTunnel` (`SceneComponent.K2_GetComponentLocation` (`/Game/InfiniteMatrix/Blueprints/BP_Tunnel.SpawnPoint` (`self.Newset Tunnel`)))))

(fn `UserConstructionScript`)